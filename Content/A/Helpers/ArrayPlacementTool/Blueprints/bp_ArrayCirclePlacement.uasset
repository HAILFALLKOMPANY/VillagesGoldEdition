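; Array placement helper that arranges static meshes in circles or arcs around the actor, with settings per array entry.
; The construction script spaces meshes by count, radius and angle limit, optionally adding a cumulative offset or yawing them toward the center.
; Meshes become hierarchical instances or separate components, and their world transforms are stored in Elements.
; The Blutility event PlaceStaticMeshes spawns a StaticMeshActor for each stored element.
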(event `PlaceStaticMeshes`
  ;[1 1 1] Convert StaticMeshComponentsto Actors
  (for _array_element (`self.Elements`)
    (bind (_staticmesh _elementlocation _elementrotation _elementscale) (break `/Game/A/Helpers/ArrayPlacementTool/Blueprints/Structures/s_ArrayPlacementElements` _array_element))
    (bind _output_get (set `self.SegmentStaticMesh` _staticmesh))
    (`/Engine/EditorBlueprintResources/StandardMacros.IsValid` _output_get
      (:`Is Valid`
        (bind _returnvalue (`|SpawnActorFromClass` "/Script/Engine.StaticMeshActor" (`KismetMathLibrary.MakeTransform` _elementlocation _elementrotation _elementscale) "AlwaysSpawn" "OverrideRootScale" null null))
        (`StaticMeshComponent.SetStaticMesh` (`StaticMeshActor.StaticMeshComponent` _returnvalue) (`self.SegmentStaticMesh`))))))

(fn `UserConstructionScript`
  (locals (CurrentStaticMesh_Local :type "StaticMesh Object Reference") (Circumference_Local :type "Float (double-precision)" :default 0.0) (SegmentDistance_Local :type "Float (double-precision)" :default 0.0) (Angle_Local :type "Float (double-precision)" :default 0.0) (ElementLocation_Locl :type "Vector Structure") (CurrentElement_Local :type Integer) (CurrentInstanceIndex_Local :type Integer :default 0))
  (bind (_returnvalue_location _returnvalue_rotation _returnvalue_scale) (`KismetMathLibrary.BreakTransform` (`SceneComponent.K2_GetComponentToWorld` (`self.NewStaticMeshComponent`))))
  (bind _outinstancetransform (`InstancedStaticMeshComponent.GetInstanceTransform` (`self.InstancedMesh`) (`local.CurrentInstanceIndex_Local`) true))
  (bind _outinstancetransform_2 (`InstancedStaticMeshComponent.GetInstanceTransform` (`self.InstancedMesh`) (`local.CurrentInstanceIndex_Local`) true))
  ;[1 1 1] For all elements do
  (for _array_element (`self.ArrayElement`)
    ;[1 1 1] SetLocalVariables
    (`|ExecutionSequence`
      (:`then_0`
        (bind (_staticmesh _circleradius _anglelimit _count _facetocenter _useconstantoffset _constantoffset _placementmethod) (break `/Game/A/Helpers/ArrayPlacementTool/Blueprints/Structures/s_ArrayCirclePlacementElement` _array_element))
        (set `self.StaticMeshElement` _staticmesh))
      (:`then_1`
        (set `self.Circle Radius` _circleradius))
      (:`then_2`
        (set `self.Count` _count))
      (:`then_3`
        (set `self.FaceToCenter` _facetocenter))
      (:`then_4`
        (set `self.UseConstantOffset` _useconstantoffset))
      (:`then_5`
        (set `self.ConstansOffset` _constantoffset))
      (:`then_6`
        (if (not (`self.UseGlobalPlacmentMethod`))
          (set `self.GlobalPlacmentMethod` _placementmethod)))
      (:`then_7`
        (set `self.AngleLimit` _anglelimit))
      (:`then_8`
        ;[1 1 1] Select Placement Method if  instanced meshes add instanc mesh component
        (switch `/Game/A/Helpers/ArrayPlacementTool/Blueprints/Enumerations/en_ArrayPlacementMethod` (`self.GlobalPlacmentMethod`)
          (:`NewEnumerator0`
            (bind _returnvalue (`AddComponent|NODE_AddHierarchicalInstancedStaticMeshComponent-0`))
            (bind _output_get (set `self.InstancedMesh` _returnvalue))
            (`StaticMeshComponent.SetStaticMesh` _output_get (`self.StaticMeshElement`)))
          (:`NewEnumerator1`
            _))
        ;[1 1 1] calculate the circumference of a circle
        (set `local.Circumference_Local` (* (* 2.0 (`KismetMathLibrary.GetPI`)) (`self.Circle Radius`)))
        ;[1 1 1] Calculate distance between elements
        (set `local.SegmentDistance_Local` (/ (`local.Circumference_Local`) (`KismetMathLibrary.Conv_IntToDouble` (`self.Count`))))
        ;[1 1 1] Calculate angel between elements
        (set `local.Angle_Local` (/ (* (`local.SegmentDistance_Local`) (`self.AngleLimit`)) (`local.Circumference_Local`)))
        ;[1 1 1] Check if static mesh is valid
        (`/Engine/EditorBlueprintResources/StandardMacros.IsValid` (`self.StaticMeshElement`)
          (:`Is Valid`
            ;[1 1 1] Add elements
            (for _index (range (`self.Count`))
              (set `local.CurrentElement_Local` _index)
              (`|ExecutionSequence`
                (:`then_0`
                  ;[1 1 1] Calculate element location
                  (bind _output_get_2 (set `local.ElementLocation_Locl` (`KismetMathLibrary.RotateAngleAxis` (`KismetMathLibrary.MakeVector` (`self.Circle Radius`)) (* (`local.CurrentElement_Local`) (`local.Angle_Local`)) (0.0 0.0 1.0))))
                  (if (`self.UseConstantOffset`)
                    (set `local.ElementLocation_Locl` (+ _output_get_2 (* (`self.ConstansOffset`) (`local.CurrentElement_Local`))))))
                (:`then_1`
                  ;[1 1 1] Select Placement Method
                  (switch `/Game/A/Helpers/ArrayPlacementTool/Blueprints/Enumerations/en_ArrayPlacementMethod` (`self.GlobalPlacmentMethod`)
                    (:`NewEnumerator0`
                      ;[1 1 1] Add instance of Static Mesh and store index
                      (bind _returnvalue_2 (`InstancedStaticMeshComponent.AddInstance` (`self.InstancedMesh`) (`KismetMathLibrary.MakeTransform` (`local.ElementLocation_Locl`))))
                      (set `local.CurrentInstanceIndex_Local` _returnvalue_2))
                    (:`NewEnumerator1`
                      ;[1 1 1] Add static mesh component and set static mesh
                      (bind _returnvalue_3 (`AddComponent|NODE_AddStaticMeshComponent-0` :`RelativeTransform` (`KismetMathLibrary.MakeTransform` (`local.ElementLocation_Locl`))))
                      (bind _output_get_3 (set `self.NewStaticMeshComponent` _returnvalue_3))
                      (`StaticMeshComponent.SetStaticMesh` _output_get_3 (`self.StaticMeshElement`)))))
                (:`then_2`
                  ;[1 1 1] In face to center true select placement method
                  (if (`self.FaceToCenter`)
                    (switch `/Game/A/Helpers/ArrayPlacementTool/Blueprints/Enumerations/en_ArrayPlacementMethod` (`self.GlobalPlacmentMethod`)
                      (:`NewEnumerator0`
                        ;[1 1 1] Rotating Instance to face center of circle
                        (`InstancedStaticMeshComponent.UpdateInstanceTransform` (`self.InstancedMesh`) (`local.CurrentInstanceIndex_Local`) (`KismetMathLibrary.MakeTransform` (.location _outinstancetransform_2) (`KismetMathLibrary.MakeRotator` 0.0 0.0 (.yaw (`KismetMathLibrary.FindLookAtRotation` (.location _outinstancetransform_2) (`SceneComponent.K2_GetComponentLocation` (`self.DefaultSceneRoot`))))) (.scale _outinstancetransform_2)) true true true))
                      (:`NewEnumerator1`
                        ;[1 1 1] Rotating Component to face center of circle
                        (`SceneComponent.K2_SetWorldRotation` (`self.NewStaticMeshComponent`) (`KismetMathLibrary.MakeRotator` 0.0 0.0 (.yaw (`KismetMathLibrary.FindLookAtRotation` (`SceneComponent.K2_GetComponentLocation` (`self.NewStaticMeshComponent`)) (`SceneComponent.K2_GetComponentLocation` (`self.DefaultSceneRoot`))))) false false)))))
                (:`then_3`
                  ;[1 1 1] Select Placement Method
                  (switch `/Game/A/Helpers/ArrayPlacementTool/Blueprints/Enumerations/en_ArrayPlacementMethod` (`self.GlobalPlacmentMethod`)
                    (:`NewEnumerator0`
                      ;[1 1 1] StoreArrayElement
                      (`KismetArrayLibrary.Array_Add` (`self.Elements`) (make `/Game/A/Helpers/ArrayPlacementTool/Blueprints/Structures/s_ArrayPlacementElements` (`self.StaticMeshElement`) (.location _outinstancetransform) (.rotation _outinstancetransform) (.scale _outinstancetransform))))
                    (:`NewEnumerator1`
                      ;[1 1 1] StoreArrayElement
                      (`KismetArrayLibrary.Array_Add` (`self.Elements`) (make `/Game/A/Helpers/ArrayPlacementTool/Blueprints/Structures/s_ArrayPlacementElements` (`self.StaticMeshElement`) _returnvalue_location _returnvalue_rotation _returnvalue_scale)))))))))))))