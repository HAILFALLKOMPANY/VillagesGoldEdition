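; Editor array-placement actor that builds repeated static mesh arrays from its ArraySettings entries.
; The construction script runs GenerateArray, spacing meshes by fixed count (constant, relative, combined or another entry's mesh-size offset) or fitting a length along X.
; AddArrayElement creates instanced or individual mesh components and records their world transforms in Elements.
; The PlaceStaticMeshes Blutility event spawns a StaticMeshActor for each recorded element.
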(event `GenerateArray`
  (bind (_currentarrayelement_staticmesh _currentarrayelement_staticmeshoffset _currentarrayelement_staticmeshrotation _currentarrayelement_elementplacementmethod _currentarrayelement_arraytype _currentarrayelement_fixedcounttype _currentarrayelement_fixedcount _currentarrayelement_fixedcountcustomoffset _currentarrayelement_fixedcountrelativeoffset _currentarrayelement_fixedcountobjectindex _currentarrayelement_objectxyzmultiply _currentarrayelement_skipfirstelement _currentarrayelement_lenght) (break `/Game/A/Helpers/ArrayPlacementTool/Blueprints/Structures/s_ArrayPlacementSegment` (`self.CurrentArrayElement`)))
  (bind _returnvalue (`StaticMesh.GetBoundingBox` (`self.StaticMesh`)))
  (bind _returnvalue_2 (`StaticMesh.GetBoundingBox` (`self.StaticMesh`)))
  ;[1 1 1] ClearElements
  (`KismetArrayLibrary.Array_Clear` (`self.Elements`))
  ;[1 1 1] for each element of elements array do ...
  (for _array_element (`self.ArraySettings`)
    ;[1 1 1] Check static mesh
    (bind _output_get (set `self.CurrentArrayElement` _array_element))
    (`/Engine/EditorBlueprintResources/StandardMacros.IsValid` (break `/Game/A/Helpers/ArrayPlacementTool/Blueprints/Structures/s_ArrayPlacementSegment` _output_get)
      (:`Is Valid`
        ;[1 1 1] SetLocalVariables
        (`|ExecutionSequence`
          (:`then_0`
            (set `self.StaticMesh` _currentarrayelement_staticmesh))
          (:`then_1`
            (set `self.StaticMeshOffset` _currentarrayelement_staticmeshoffset))
          (:`then_2`
            (set `self.StaticMeshRotation` _currentarrayelement_staticmeshrotation))
          (:`then_3`
            ;;[1 1 1] Set only if UseGlobalPlacmentMethod == false
            (if (not (`self.UseGlobalPlacmentMethod`))
              (set `self.GlobalPlacementMethod` _currentarrayelement_elementplacementmethod)))
          (:`then_4`
            (set `self.ArrayType` _currentarrayelement_arraytype))
          (:`then_5`
            (set `self.FixedCountType` _currentarrayelement_fixedcounttype))
          (:`then_6`
            (set `self.FixedCount` _currentarrayelement_fixedcount))
          (:`then_7`
            (set `self.ConstantOffset` _currentarrayelement_fixedcountcustomoffset))
          (:`then_8`
            (set `self.RelativeOffset` _currentarrayelement_fixedcountrelativeoffset))
          (:`then_9`
            (set `self.ObjectOffsetIndex` _currentarrayelement_fixedcountobjectindex))
          (:`then_10`
            (set `self.ObjectMultiply` _currentarrayelement_objectxyzmultiply))
          (:`then_11`
            (set `self.SkipFirstElement` _currentarrayelement_skipfirstelement))
          (:`then_12`
            (set `self.Length` _currentarrayelement_lenght))
          (:`then_13`
            ;[1 1 1] Select Placment Method
            (switch `/Game/A/Helpers/ArrayPlacementTool/Blueprints/Enumerations/en_ArrayPlacementMethod` (`self.GlobalPlacementMethod`)
              (:`NewEnumerator0`
                ;[1 1 1] Add Instanced Static Mesh Component
                (bind _returnvalue_3 (`AddComponent|NODE_AddInstancedStaticMeshComponent-0`))
                (set `self.InstancStaticMesh` _returnvalue_3)
                (`StaticMeshComponent.SetStaticMesh` (`self.InstancStaticMesh`) (`self.StaticMesh`)))
              (:`NewEnumerator1`
                _))
            ;[1 1 1] Select Array Type
            (switch `/Game/A/Helpers/ArrayPlacementTool/Blueprints/Enumerations/en_ArrayPlacementType` (`self.ArrayType`)
              (:`NewEnumerator0`
                ;[1 1 1] fixed count method selection
                (switch `/Game/A/Helpers/ArrayPlacementTool/Blueprints/Enumerations/en_ArrayPlacementFixedCountType` (`self.FixedCountType`)
                  (:`NewEnumerator0`
                    ;[1 1 1] Fixed count constant offset method
                    ;;[1 1 1] Calculate location, rotation and add element
                    (for _index (range (`KismetMathLibrary.SelectInt` 1 0 (`self.SkipFirstElement`)) (`self.FixedCount`))
                      (`self.AddArrayElement` (+ (* (`self.ConstantOffset`) _index) (`self.StaticMeshOffset`)) (`self.StaticMeshRotation`) (`self.GetActorScale3D`))))
                  (:`NewEnumerator1`
                    ;[1 1 1] Fix count relative offset
                    ;;[1 1 1] Calculate location, rotation and add element
                    (for _index_2 (range (`KismetMathLibrary.SelectInt` 1 0 (`self.SkipFirstElement`)) (`self.FixedCount`))
                      (`self.AddArrayElement` (+ (* (* (`self.RelativeOffset`) (`/Game/A/Helpers/ArrayPlacementTool/Blueprints/bpfl_ArrayPlacement.GetStaticMeshSize` (`self.StaticMesh`))) _index_2) (`self.StaticMeshOffset`)) (`self.StaticMeshRotation`) (`self.GetActorScale3D`))))
                  (:`NewEnumerator2`
                    ;[1 1 1] Fixed count relative and constant offset
                    ;;[1 1 1] Calculate location, rotation and add element
                    (for _index_3 (range (`KismetMathLibrary.SelectInt` 1 0 (`self.SkipFirstElement`)) (`self.FixedCount`))
                      (`self.AddArrayElement` (+ (+ (* (`self.ConstantOffset`) _index_3) (* (* (`self.RelativeOffset`) (`/Game/A/Helpers/ArrayPlacementTool/Blueprints/bpfl_ArrayPlacement.GetStaticMeshSize` (`self.StaticMesh`))) _index_3)) (`self.StaticMeshOffset`)) (`self.StaticMeshRotation`) (`self.GetActorScale3D`))))
                  (:`NewEnumerator3`
                    ;[1 1 1] Fixed ount object offset
                    ;;[1 1 1] Check array element
                    (if (`KismetArrayLibrary.Array_IsValidIndex` (`self.ArraySettings`) (`self.ObjectOffsetIndex`))
                      ;;[1 1 1] Calculate location, rotation and add element
                      (for _index_4 (range (`KismetMathLibrary.SelectInt` 1 0 (`self.SkipFirstElement`)) (`self.FixedCount`))
                        (`self.AddArrayElement` (+ (`self.StaticMeshOffset`) (* (* (`self.ObjectMultiply`) (`/Game/A/Helpers/ArrayPlacementTool/Blueprints/bpfl_ArrayPlacement.GetStaticMeshSize` (`.StaticMesh_30_3A347D65462244E3D62F13B107B92973` (break `/Game/A/Helpers/ArrayPlacementTool/Blueprints/Structures/s_ArrayPlacementSegment` (`|GetArrayItem` (`self.ArraySettings`) (`self.ObjectOffsetIndex`)))))) _index_4)) (`self.StaticMeshRotation`) (`self.GetActorScale3D`)))))))
              (:`NewEnumerator1`
                ;[1 1 1] Fit Length placment method
                ;;[1 1 1] Calculate location, rotation and add element
                (for _index_5 (range (`KismetMathLibrary.FCeil` (/ (`self.Length`) (+ (`KismetMathLibrary.Abs` (.x (break `Box` _returnvalue_2))) (`KismetMathLibrary.Abs` (.x (`.Max` (break `Box` _returnvalue_2))))))))
                  (`self.AddArrayElement` (+ (`KismetMathLibrary.MakeVector` (* _index_5 (+ (`KismetMathLibrary.Abs` (.x (break `Box` _returnvalue))) (`KismetMathLibrary.Abs` (.x (`.Max` (break `Box` _returnvalue))))))) (`self.StaticMeshOffset`)) (`self.StaticMeshRotation`) (`self.GetActorScale3D`)))))))))))

(event `PlaceStaticMeshes`
  ;[1 1 1] Convert StaticMeshComponentsto Actors
  (for _array_element (`self.Elements`)
    (bind (_staticmesh _elementlocation _elementrotation _elementscale) (break `/Game/A/Helpers/ArrayPlacementTool/Blueprints/Structures/s_ArrayPlacementElements` _array_element))
    (bind _output_get (set `self.SegmentStaticMesh` _staticmesh))
    (`/Engine/EditorBlueprintResources/StandardMacros.IsValid` _output_get
      (:`Is Valid`
        (bind _returnvalue (`|SpawnActorFromClass` "/Script/Engine.StaticMeshActor" (`KismetMathLibrary.MakeTransform` _elementlocation _elementrotation _elementscale) "AlwaysSpawn" "OverrideRootScale" null null))
        (`StaticMeshComponent.SetStaticMesh` (`StaticMeshActor.StaticMeshComponent` _returnvalue) (`self.SegmentStaticMesh`))))))

(fn `AddArrayElement`
  (params (RelativeLocation :type "Vector Structure") (RelativeRotation :type "Rotator Structure") (Scale :type "Vector Structure"))
  (locals (RelativeLocation_Local :type "Vector Structure") (RelativeRotation_Local :type "Rotator Structure") (Scale_Local :type "Vector Structure") (NewStaticMeshComponent_Local :type "StaticMeshComponent Object Reference"))
  (bind (_returnvalue_location _returnvalue_rotation _returnvalue_scale) (`KismetMathLibrary.BreakTransform` (`SceneComponent.K2_GetComponentToWorld` (`local.NewStaticMeshComponent_Local`))))
  ;[1 1 1] Set local variables
  (set `local.RelativeLocation_Local` RelativeLocation)
  (set `local.RelativeRotation_Local` RelativeRotation)
  (set `local.Scale_Local` Scale)
  ;[1 1 1] SelectPlacmentMethod
  (switch `/Game/A/Helpers/ArrayPlacementTool/Blueprints/Enumerations/en_ArrayPlacementMethod` (`self.GlobalPlacementMethod`)
    (:`NewEnumerator0`
      ;[1 1 1] AddStaticMeshInstance
      (bind _returnvalue (`InstancedStaticMeshComponent.AddInstance` (`self.InstancStaticMesh`) (`KismetMathLibrary.MakeTransform` (`local.RelativeLocation_Local`) (`local.RelativeRotation_Local`) (`local.Scale_Local`))))
      (bind _outinstancetransform (`InstancedStaticMeshComponent.GetInstanceTransform` (`self.InstancStaticMesh`) _returnvalue true))
      ;[1 1 1] StoreArrayElement
      (`KismetArrayLibrary.Array_Add` (`self.Elements`) (make `/Game/A/Helpers/ArrayPlacementTool/Blueprints/Structures/s_ArrayPlacementElements` (`self.StaticMesh`) (.location _outinstancetransform) (.rotation _outinstancetransform) (.scale _outinstancetransform))))
    (:`NewEnumerator1`
      ;[1 1 1] AddStaticmeshComponent
      (bind _returnvalue_2 (`AddComponent|NODE_AddStaticMeshComponent-0` :`RelativeTransform` (`KismetMathLibrary.MakeTransform` (`local.RelativeLocation_Local`) (`local.RelativeRotation_Local`) (`local.Scale_Local`))))
      (bind _output_get (set `local.NewStaticMeshComponent_Local` _returnvalue_2))
      (`StaticMeshComponent.SetStaticMesh` _output_get (`self.StaticMesh`))
      ;[1 1 1] StoreArrayElement
      (`KismetArrayLibrary.Array_Add` (`self.Elements`) (make `/Game/A/Helpers/ArrayPlacementTool/Blueprints/Structures/s_ArrayPlacementElements` (`self.StaticMesh`) _returnvalue_location _returnvalue_rotation _returnvalue_scale)))))

(fn `UserConstructionScript`
  (`self.GenerateArray`))