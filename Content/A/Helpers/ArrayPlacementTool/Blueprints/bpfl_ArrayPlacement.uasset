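; Blueprint function library for the array placement tool helper, providing a static mesh measurement function.
; GetStaticMeshSize reads the mesh's bounding box and returns separate X, Y and Z sizes.
; Each size sums the absolute min and max on that axis, so it matches the true extent only when the bounds span the mesh origin.
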(fn `GetStaticMeshSize`
  (params (StaticMesh :type "StaticMesh Object Reference"))
  (returns (StaticMeshSize :type "Vector Structure"))
  (bind _returnvalue (`StaticMesh.GetBoundingBox` StaticMesh))
  (return (`KismetMathLibrary.MakeVector` (+ (`KismetMathLibrary.Abs` (.x (break `Box` _returnvalue))) (`KismetMathLibrary.Abs` (.x (`.Max` (break `Box` _returnvalue))))) (+ (`KismetMathLibrary.Abs` (.y (break `Box` _returnvalue))) (`KismetMathLibrary.Abs` (.y (`.Max` (break `Box` _returnvalue))))) (+ (`KismetMathLibrary.Abs` (.z (break `Box` _returnvalue))) (`KismetMathLibrary.Abs` (.z (`.Max` (break `Box` _returnvalue))))))))