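; Spline array placement tool that lays out static meshes along a spline, rebuilt in the construction script.
; For each array setting, GenerateArray places elements at spline points, evenly by count, or at a fixed spacing, with optional tangent rotation and end skipping.
; AddArrayElement creates instanced or individual mesh components and records world transforms in Elements.
; The PlaceStaticMeshes Blutility event spawns separate StaticMeshActors from those records.
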(event `GenerateArray`
  (bind (_currentarrayelement_staticmesh _currentarrayelement_staticmeshoffset _currentarrayelement_placementmethod _currentarrayelement_splineelementcount _currentarrayelement_splineplacmenttype _currentarrayelement_distance _currentarrayelement_skipfirstelement _currentarrayelement_skiplastelement _currentarrayelement_splineelementrotate) (break `/Game/A/Helpers/ArrayPlacementTool/Blueprints/Structures/s_ArraySplinePlacementSegment` (`self.CurrentArrayElement`)))
  ;[1 1 1] ClearElements
  (`KismetArrayLibrary.Array_Clear` (`self.Elements`))
  ;[1 1 1] for each element of elements array do ...
  (for _array_element (`self.ArraySettings`)
    ;[1 1 1] Check static mesh
    (`/Engine/EditorBlueprintResources/StandardMacros.IsValid` (`.StaticMesh_30_3A347D65462244E3D62F13B107B92973` (break `/Game/A/Helpers/ArrayPlacementTool/Blueprints/Structures/s_ArraySplinePlacementSegment` _array_element))
      (:`Is Valid`
        (set `self.CurrentArrayElement` _array_element)
        ;[1 1 1] SetLocalVariables
        (`|ExecutionSequence`
          (:`then_0`
            (set `self.StaticMesh` _currentarrayelement_staticmesh))
          (:`then_1`
            (set `self.StaticMeshOffset` _currentarrayelement_staticmeshoffset))
          (:`then_2`
            (set `self.StaticMeshRotation` (struct)))
          (:`then_3`
            ;;[1 1 1] Set only if UseGlobalPlacmentMethod == false
            (if (not (`self.UseGlobalPlacmentMethod`))
              (set `self.GlobalPlacementMethod` _currentarrayelement_placementmethod)))
          (:`then_4`
            (set `self.SplineElementCount` _currentarrayelement_splineelementcount))
          (:`then_5`
            (set `self.SplinePlacmentType` _currentarrayelement_splineplacmenttype))
          (:`then_6`
            (set `self.Distance` _currentarrayelement_distance))
          (:`then_7`
            (set `self.SkipLastElement` _currentarrayelement_skiplastelement))
          (:`then_8`
            (set `self.SkipFirstElement` _currentarrayelement_skipfirstelement))
          (:`then_9`
            (set `self.SplineElementRotate` _currentarrayelement_splineelementrotate))
          (:`then_10`
            ;[1 1 1] Select Placment Method
            (switch `/Game/A/Helpers/ArrayPlacementTool/Blueprints/Enumerations/en_ArrayPlacementMethod` (`self.GlobalPlacementMethod`)
              (:`NewEnumerator0`
                ;[1 1 1] Add Instanced Static Mesh Component
                (bind _returnvalue (`AddComponent|NODE_AddInstancedStaticMeshComponent-0`))
                (set `self.InstancStaticMesh` _returnvalue)
                (`StaticMeshComponent.SetStaticMesh` (`self.InstancStaticMesh`) (`self.StaticMesh`)))
              (:`NewEnumerator1`
                _))
            ;[1 1 1] Check if the spline component is valid than select lacment method
            (`/Engine/EditorBlueprintResources/StandardMacros.IsValid` (`self.Spline`)
              (:`Is Valid`
                (switch `/Game/A/Helpers/ArrayPlacementTool/Blueprints/Enumerations/en_ArrayPlacmentSplinePlacementType` (`self.SplinePlacmentType`)
                  (:`NewEnumerator0`
                    ;[1 1 1] Add element at point
                    ;;[1 1 1] Calculate rotation,location and add element
                    (for _index (range (`KismetMathLibrary.SelectInt` 1 0 (`self.SkipFirstElement`)) (+ (- (`SplineComponent.GetNumberOfSplinePoints` (`self.Spline`)) (`KismetMathLibrary.SelectInt` 2 1 (`self.SkipLastElement`))) 1))
                      (bind (_location _tangent) (`SplineComponent.GetLocationAndTangentAtSplinePoint` (`self.Spline`) _index "Local"))
                      (`self.AddArrayElement` (+ _location (`self.StaticMeshOffset`)) (`KismetMathLibrary.Conv_VectorToRotator` (`KismetMathLibrary.SelectVector` _tangent (0.0 0.0 0.0) (`self.SplineElementRotate`))) (`self.GetActorScale3D`))))
                  (:`NewEnumerator1`
                    ;[1 1 1] Add element count equal distance at spline
                    ;;[1 1 1] Calculate distance between element
                    (set `self.Distance` (/ (`SplineComponent.GetSplineLength` (`self.Spline`)) (`KismetMathLibrary.Conv_IntToDouble` (- (`self.SplineElementCount`) 1))))
                    ;;[1 1 1] Calculate rotation,location and add element
                    (for _index_2 (range (`KismetMathLibrary.SelectInt` 1 0 (`self.SkipFirstElement`)) (+ (- (`self.SplineElementCount`) (`KismetMathLibrary.SelectInt` 2 1 (`self.SkipLastElement`))) 1))
                      (bind _returnvalue_2 (* _index_2 (`self.Distance`)))
                      (`self.AddArrayElement` (+ (`SplineComponent.GetLocationAtDistanceAlongSpline` (`self.Spline`) _returnvalue_2 "Local") (`self.StaticMeshOffset`)) (`KismetMathLibrary.Conv_VectorToRotator` (`KismetMathLibrary.SelectVector` (`SplineComponent.GetTangentAtDistanceAlongSpline` (`self.Spline`) _returnvalue_2 "Local") (0.0 0.0 0.0) (`self.SplineElementRotate`))) (`self.GetActorScale3D`))))
                  (:`NewEnumerator2`
                    ;[1 1 1] Add element count custom distance at spline
                    ;;[1 1 1] Store Spline Length
                    (set `self.SplineLength_Local` (`SplineComponent.GetSplineLength` (`self.Spline`)))
                    ;;[1 1 1] Calculate rotation,location and add element
                    (for _index_3 (range (`KismetMathLibrary.SelectInt` 1 0 (`self.SkipFirstElement`)) (+ (- (`self.SplineElementCount`) (`KismetMathLibrary.SelectInt` 2 1 (`self.SkipLastElement`))) 1))
                      ;;;[1 1 1] check if distance is not bigger than spline length
                      (bind _output_get (set `self.CurentElementDistance` (* _index_3 (`self.Distance`))))
                      (if (> (`self.SplineLength_Local`) _output_get)
                        (`self.AddArrayElement` (+ (`SplineComponent.GetLocationAtDistanceAlongSpline` (`self.Spline`) (`self.CurentElementDistance`) "Local") (`self.StaticMeshOffset`)) (`KismetMathLibrary.Conv_VectorToRotator` (`KismetMathLibrary.SelectVector` (`SplineComponent.GetTangentAtDistanceAlongSpline` (`self.Spline`) (`self.CurentElementDistance`) "Local") (0.0 0.0 0.0) (`self.SplineElementRotate`))) (`self.GetActorScale3D`))))))))))))))

(event `PlaceStaticMeshes`
  ;[1 1 1] Convert StaticMeshComponentsto Actors
  (for _array_element (`self.Elements`)
    (bind (_staticmesh _elementlocation _elementrotation _elementscale) (break `/Game/A/Helpers/ArrayPlacementTool/Blueprints/Structures/s_ArrayPlacementElements` _array_element))
    (bind _output_get (set `self.SegmentStaticMesh` _staticmesh))
    (`/Engine/EditorBlueprintResources/StandardMacros.IsValid` _output_get
      (:`Is Valid`
        (bind _returnvalue (`|SpawnActorFromClass` "/Script/Engine.StaticMeshActor" (`KismetMathLibrary.MakeTransform` _elementlocation _elementrotation _elementscale) "AlwaysSpawn" "OverrideRootScale" null null))
        (`StaticMeshComponent.SetStaticMesh` (`StaticMeshActor.StaticMeshComponent` _returnvalue) (`self.SegmentStaticMesh`))))))

(fn `AddArrayElement`
  (params (RelativeLocation :type "Vector Structure") (RelativeRotation :type "Rotator Structure") (Scale :type "Vector Structure"))
  (locals (RelativeLocation_Local :type "Vector Structure") (RelativeRotation_Local :type "Rotator Structure") (Scale_Local :type "Vector Structure") (NewStaticMeshComponent_Local :type "StaticMeshComponent Object Reference"))
  (bind (_returnvalue_location _returnvalue_rotation _returnvalue_scale) (`KismetMathLibrary.BreakTransform` (`SceneComponent.K2_GetComponentToWorld` (`local.NewStaticMeshComponent_Local`))))
  ;[1 1 1] Set local variables
  (set `local.RelativeLocation_Local` RelativeLocation)
  (set `local.RelativeRotation_Local` RelativeRotation)
  (set `local.Scale_Local` Scale)
  ;[1 1 1] SelectPlacmentMethod
  (switch `/Game/A/Helpers/ArrayPlacementTool/Blueprints/Enumerations/en_ArrayPlacementMethod` (`self.GlobalPlacementMethod`)
    (:`NewEnumerator0`
      ;[1 1 1] AddStaticMeshInstance
      (bind _returnvalue (`InstancedStaticMeshComponent.AddInstance` (`self.InstancStaticMesh`) (`KismetMathLibrary.MakeTransform` (`local.RelativeLocation_Local`) (`local.RelativeRotation_Local`) (`local.Scale_Local`))))
      (bind _outinstancetransform (`InstancedStaticMeshComponent.GetInstanceTransform` (`self.InstancStaticMesh`) _returnvalue true))
      ;[1 1 1] StoreArrayElement
      (`KismetArrayLibrary.Array_Add` (`self.Elements`) (make `/Game/A/Helpers/ArrayPlacementTool/Blueprints/Structures/s_ArrayPlacementElements` (`self.StaticMesh`) (.location _outinstancetransform) (.rotation _outinstancetransform) (.scale _outinstancetransform))))
    (:`NewEnumerator1`
      ;[1 1 1] AddStaticmeshComponent
      (bind _returnvalue_2 (`AddComponent|NODE_AddStaticMeshComponent-0` :`RelativeTransform` (`KismetMathLibrary.MakeTransform` (`local.RelativeLocation_Local`) (`local.RelativeRotation_Local`) (`local.Scale_Local`))))
      (bind _output_get (set `local.NewStaticMeshComponent_Local` _returnvalue_2))
      (`StaticMeshComponent.SetStaticMesh` _output_get (`self.StaticMesh`))
      ;[1 1 1] StoreArrayElement
      (`KismetArrayLibrary.Array_Add` (`self.Elements`) (make `/Game/A/Helpers/ArrayPlacementTool/Blueprints/Structures/s_ArrayPlacementElements` (`self.StaticMesh`) _returnvalue_location _returnvalue_rotation _returnvalue_scale)))))

(fn `UserConstructionScript`
  (`self.GenerateArray`))