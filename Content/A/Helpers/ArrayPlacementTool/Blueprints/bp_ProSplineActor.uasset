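; Spline placement actor that builds meshes along its spline in the construction script from an array of segment definitions, each with its own offset and meshes.
; For every segment, it stretches a spline mesh between each pair of neighboring points, applying the configured collision type and blocking all channels.
; Optional static meshes are placed at interior points, oriented along the tangent, and as start and end caps at the spline's ends.
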(fn `UserConstructionScript`
  (bind _currentsplinemeshcomponent (`self.CurrentSplineMeshComponent`))
  (bind (_location _tangent) (`SplineComponent.GetLocationAndTangentAtSplinePoint` (`self.Spline`) (`self.CurrentPintIndex`) "Local"))
  (bind (_location_2 _tangent_2) (`SplineComponent.GetLocationAndTangentAtSplinePoint` (`self.Spline`) (`self.CurrentPintIndex`) "Local"))
  (bind _returnvalue (- (`self.NumberOfSplinePoints`) 1))
  (bind (_location_3 _tangent_3) (`SplineComponent.GetLocationAndTangentAtSplinePoint` (`self.Spline`) (+ (`self.CurrentPintIndex`) 1) "Local"))
  ;[1 1 1] Get and store number of spline points
  (set `self.NumberOfSplinePoints` (`SplineComponent.GetNumberOfSplinePoints` (`self.Spline`)))
  ;[1 1 1] For each Segment in array do ....
  (for _array_element (`self.SegmentsArray`)
    (bind (_segmentoffset _splinemesh _startcupmesh _endcupmesh _extrapointmesh) (break `/Game/A/Helpers/ArrayPlacementTool/Blueprints/Structures/s_SmartSpline_Segment` _array_element))
    ;[1 1 1] Get element and set local variables
    (set `self.SegmentOffset` _segmentoffset)
    (set `self.SplineMesh` _splinemesh)
    (set `self.Spline MeshStartCap` _startcupmesh)
    (set `self.SplineMeshEndCap` _endcupmesh)
    (set `self.ExtraPointMesh` _extrapointmesh)
    ;[1 1 1] Add mesh component between spline points / Loop from first point to Last -1
    (for _index (range (+ (- (`self.NumberOfSplinePoints`) 2) 1))
      (set `self.CurrentPintIndex` _index)
      (`|ExecutionSequence`
        (:`then_0`
          ;[1 1 1] Get and store location of current point
          (set `self.CurrentPointLocation` (+ (`self.SegmentOffset`) _location))
          (set `self.CurrentPointTangent` _tangent)
          ;[1 1 1] Get and store location of next point
          (set `self.NextPointLocation` (+ (`self.SegmentOffset`) _location_3))
          (set `self.NextPointTangent` _tangent_3))
        (:`then_1`
          ;[1 1 1] Check spline mesh
          (`/Engine/EditorBlueprintResources/StandardMacros.IsValid` (`self.SplineMesh`)
            (:`Is Valid`
              ;[1 1 1] Add spline mesh component and setup static mesh
              (bind _returnvalue_2 (`AddComponent|NODE_AddSplineMeshComponent-0`))
              (bind _output_get (set `self.CurrentSplineMeshComponent` _returnvalue_2))
              (`StaticMeshComponent.SetStaticMesh` _output_get (`self.SplineMesh`))
              ;[1 1 1] Set spline mest component parameters
              (`SplineMeshComponent.SetStartAndEnd` (`self.CurrentSplineMeshComponent`) (`self.CurrentPointLocation`) (`self.CurrentPointTangent`) (`self.NextPointLocation`) (`self.NextPointTangent`) true)
              ;[1 1 1] Enable Collisions for splinemesh component
              (`PrimitiveComponent.SetCollisionEnabled` _currentsplinemeshcomponent (`self.CollisionType`))
              (`PrimitiveComponent.SetCollisionResponseToAllChannels` _currentsplinemeshcomponent "ECR_Block"))))
        (:`then_2`
          ;[1 1 1] Check when add extra mesh at point
          (if (and (`KismetSystemLibrary.IsValid` (`self.ExtraPointMesh`)) (!= (`self.CurrentPintIndex`) 0))
            ;[1 1 1] Add extra mesh at spline oint
            (bind _returnvalue_3 (`AddComponent|NODE_AddStaticMeshComponent-2` :`RelativeTransform` (`KismetMathLibrary.MakeTransform` (+ (`self.SegmentOffset`) _location_2) (`KismetMathLibrary.Conv_VectorToRotator` _tangent_2))))
            (`StaticMeshComponent.SetStaticMesh` _returnvalue_3 (`self.ExtraPointMesh`))))))
    (`|ExecutionSequence`
      (:`then_0`
        ;[1 1 1] Get and store location of first point
        (`self.Spline MeshStartCap`
          (:`then`
            (set `self.FirstPointLocation` (+ (`self.SegmentOffset`) (`SplineComponent.GetLocationAtSplinePoint` (`self.Spline`) 0 "Local")))
            (set `self.FirstPointTangent` (`SplineComponent.GetRotationAtSplinePoint` (`self.Spline`) 0 "Local"))
            ;[1 1 1] Add spline start and end cups
            (bind _returnvalue_4 (`AddComponent|NODE_AddStaticMeshComponent-0` :`RelativeTransform` (`KismetMathLibrary.MakeTransform` (`self.FirstPointLocation`) (`self.FirstPointTangent`))))
            (`StaticMeshComponent.SetStaticMesh` _returnvalue_4 (`self.Spline MeshStartCap`)))
          (:`else`)))
      (:`then_1`
        ;[1 1 1] Get and store location of last point
        (`self.SplineMeshEndCap`
          (:`then`
            (set `self.LastPointLocation` (+ (`self.SegmentOffset`) (`SplineComponent.GetLocationAtSplinePoint` (`self.Spline`) _returnvalue "Local")))
            (set `self.LastPointTangent` (`SplineComponent.GetRotationAtSplinePoint` (`self.Spline`) _returnvalue "Local"))
            ;[1 1 1] Add spline start and end cups
            (bind _returnvalue_5 (`AddComponent|NODE_AddStaticMeshComponent-1` :`RelativeTransform` (`KismetMathLibrary.MakeTransform` (`self.LastPointLocation`) (`self.LastPointTangent`))))
            (`StaticMeshComponent.SetStaticMesh` _returnvalue_5 (`self.SplineMeshEndCap`)))
          (:`else`))))))